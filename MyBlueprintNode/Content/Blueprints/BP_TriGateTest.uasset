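; BP_TriGateTest is a test Blueprint for the TriGate node, which branches an integer to Positive, Zero or Negative outputs.
; Pressing 3 feeds each element of IntArray through TriGate, while pressing 4 feeds it ten random integers spanning negative and positive values.
; Each output calls the PrintMessage helper, which prints the value with its sign label.
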(event Input|KeyboardEvents|4
  (params (Key :type Key%20Structure))
  ;[1 1 1] Test Random
  (:Pressed
    (for _index (range 0 9)
      (bind _output_get (Variables|Default|SetRand (Math|Random|RandomIntegerinRange -100 100)))
      (|TriGate _output_get
        (:Positive
          (CallFunction|PrintMessage _output_get "Positive"))
        (:Zero
          (CallFunction|PrintMessage _output_get "Zero"))
        (:Negative
          (CallFunction|PrintMessage _output_get "Negative"))))))

(event Input|KeyboardEvents|3
  (params (Key :type Key%20Structure))
  ;[1 1 1] Test Array
  (:Pressed
    (for _array_element (Variables|Default|GetIntArray)
      (|TriGate _array_element
        (:Positive
          (CallFunction|PrintMessage _array_element "Positive"))
        (:Zero
          (CallFunction|PrintMessage _array_element "Zero"))
        (:Negative
          (CallFunction|PrintMessage _array_element "Negative"))))))

(fn ConstructionScript)

(fn PrintMessage
  (params (Input :type Integer) (Message :type String))
  (Development|PrintText (Utilities|Text|FormatText "{0} {1}" Input (Utilities|Text|ToText(String) Message))))