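; BP_FocusActor_HUD is a HUD Blueprint for the FocusActor content that draws a crosshair at the center of the screen.
; On each DrawHUD event it draws the T_Crosshair texture with an orange tint, as a square sized by CrosshairSize.
; Math Expression nodes compute each screen coordinate as half the screen size minus half the icon size, keeping the crosshair centered at any resolution.
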(event EventDrawHUD
  (params (SizeX :type Integer) (SizeY :type Integer))
  (bind _crosshairsize (Variables|Default|GetCrosshairSize))
  ;[1 1 1] Draw Crosshair
  (Canvas|DrawTexture "/Game/Assets/UI/T_Crosshair.T_Crosshair" (|((ScreenSize/2)-(IconSize/2)) (Math|Conversions|ToFloat(Integer) SizeX) _crosshairsize) (|((ScreenSize/2)-(IconSize/2)) (Math|Conversions|ToFloat(Integer) SizeY) _crosshairsize) _crosshairsize _crosshairsize 0.0 0.0 1.0 1.0 "(R=1.000000,G=0.339176,B=0.107139,A=1.000000)"))

(fn ConstructionScript)