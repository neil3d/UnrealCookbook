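; BP_SplinePipe is a spline-driven actor that builds a pipe from deformed mesh segments along its spline.
; The Construction Script loops over adjacent spline points, adding a manually attached Spline Mesh component for each segment.
; Each segment's start and end positions and tangents come from its two bounding points, sampled in world space.
; The event graph holds only disabled placeholder events, so there is no runtime logic.
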(event EventBeginPlay)

(event Collision|EventActorBeginOverlap
  (params (OtherActor :type Actor%20Object%20Reference)))

(event EventTick
  (params (DeltaSeconds :type Float%20%28single-precision%29)))

(fn ConstructionScript
  (bind _spline (Variables|Default|GetSpline))
  ;[1 1 1] Add Splie Mesh on each sigment of spline
  (for _index (range 1 (- (Spline|GetNumberOfSplinePoints (Variables|Default|GetSpline)) 1))
    (bind _returnvalue (AddComponent|AddSplineMeshComponent true))
    (Class|SceneComponent|Attachto (Variables|Default|GetDefaultSceneRoot) 0 "None" "KeepRelativeOffset" true)
    (SplineMesh|SetStartandEnd _returnvalue (.Location (Spline|GetLocationandTangentatSplinePoint _spline (- _index 1) "World")) (.Tangent (Spline|GetLocationandTangentatSplinePoint _spline (- _index 1) "World")) (.Location (Spline|GetLocationandTangentatSplinePoint _spline _index "World")) (.Tangent (Spline|GetLocationandTangentatSplinePoint _spline _index "World")) true :!class /Script/Engine.SplineMeshComponent)))