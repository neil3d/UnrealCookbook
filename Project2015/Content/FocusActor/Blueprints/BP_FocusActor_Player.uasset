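; Player Blueprint that detects which focusable actor the player is looking at and notifies it.
; Each Tick runs a 2000-unit visibility line trace from the eyes viewpoint, passing hits that implement BPI_FocusAction to OnFocusActor.
; On a change of target, it calls LostFocus on the previous actor and OnFocus on the new one.
; A miss or non-focusable hit leaves the current focus in place.
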(event Custom|OnFocusActor
  (params (Actor :type Actor%20Object%20Reference))
  ;[1 1 1] Check Focus Actor Change
  (if (!= Actor (Variables|Default|GetFocusActor))
    (Utilities|FlowControl|Sequence
      (:then_0
        (Utilities|IsValid (Variables|Default|GetFocusActor)
          (:Is%20Valid
            (bind _asbpi_focus_action (Utilities|Casting|CastToBPI_FocusAction (Variables|Default|GetFocusActor)))
            (Default|LostFocus _asbpi_focus_action))))
      (:then_1
        (bind _output_get (Variables|Default|SetFocusActor Actor))
        (bind _asbpi_focus_action_2 (Utilities|Casting|CastToBPI_FocusAction _output_get))
        (Default|OnFocus _asbpi_focus_action_2)))))

(event EventTick
  (params (DeltaSeconds :type Float%20%28single-precision%29))
  (bind (_outlocation _outrotation) (Actor|GetActorEyesViewPoint))
  ;[1 1 1] LineTrace on Tick
  (bind (_outhit _returnvalue) (Collision|LineTraceByChannel _outlocation (+ _outlocation (* (Math|Vector|GetForwardVector _outrotation) 2e+03)) "TraceTypeQuery1" false 0 "None"))
  (if _returnvalue
    (if (Utilities|DoesObjectImplementInterface (.HitActor (Collision|BreakHitResult _outhit)) "/Game/FocusActor/Blueprints/BPI_FocusAction.BPI_FocusAction_C")
      (CallFunction|OnFocusActor (.HitActor (Collision|BreakHitResult _outhit))))))

(fn ConstructionScript)