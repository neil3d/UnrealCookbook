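; BP_MyDoor is an interactable door that swings open and shut while changing color.
; Each Interact flips between playing and reversing a timeline, whose alpha rotates the door mesh and blends its material color from yellow to red.
; The construction script creates the dynamic material instance used for the tint.
; The Closed flag tracks the toggle, but GetState always returns false, and BeginPlay only prints a delayed debug greeting.
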(event EventInteract
  (Utilities|FlowControl|FlipFlop
    (:A
      (Variables|Default|SetClosed false)
      (bind _alpha (Timeline|Timeline_0 Play)
        (:Update
          (Utilities|FlowControl|Sequence
            (:then_0
              (Transformation|SetRelativeRotation (Variables|Default|GetSM_Door) (Math|Rotator|Lerp(Rotator) "0, 0, 0" "0,100.000000, 0" _alpha) false false))
            (:then_1
              (Rendering|Material|SetVectorParameterValue (Variables|Default|GetMyMtl) "Color" (Math|Color|Lerp(LinearColor) "(R=0.989583,G=0.825564,B=0.194250,A=1.000000)" "(R=0.942708,G=0.009820,B=0.060381,A=1.000000)" _alpha) :!class /Script/Engine.MaterialInstanceDynamic))))))
    (:B
      (Variables|Default|SetClosed true)
      (Timeline|Timeline_0 Reverse))))

(event EventBeginPlay
  (Utilities|FlowControl|Delay 0.2)
  (Development|PrintString "Hello"))

(fn ConstructionScript
  (bind _returnvalue (Rendering|Material|CreateDynamicMaterialInstance (Variables|Default|GetSM_Door) 0 0 "None" :!class /Script/Engine.PrimitiveComponent))
  (Variables|Default|SetMyMtl _returnvalue))

(fn GetState
  (return false))