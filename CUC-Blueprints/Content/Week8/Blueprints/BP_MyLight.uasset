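; BP_MyLight is a light actor that the player or other logic can toggle through an Interact event.
; On BeginPlay it finds a BP_MyPowerSwitch in the level and binds to its PowerOff dispatcher.
; Both power-off and Interact call ToggleLight, so power-off flips the light rather than forcing it off.
; A FlipFlop, turning off first, sets the point light's intensity and the On flag that GetState returns.
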(event Custom|ToggleLight
  (bind _pointlight (Variables|Default|GetPointLight))
  ;[1 1 1] Toggle Light
  (Utilities|FlowControl|FlipFlop
    (:A
      (Variables|Default|SetOn false)
      (Rendering|Components|Light|SetIntensity _pointlight 0.0))
    (:B
      (Variables|Default|SetOn true)
      (Rendering|Components|Light|SetIntensity _pointlight 5e+03))))

(event Custom|OnPowerOff
  ;[1 1 1] Comment
  (CallFunction|ToggleLight))

(event EventInteract
  (CallFunction|ToggleLight))

(event EventBeginPlay
  ;[1 1 1] Comment
  (bind _returnvalue (Actor|GetActorOfClass "/Game/Week8/Blueprints/BP_MyPowerSwitch.BP_MyPowerSwitch_C"))
  (Utilities|IsValid _returnvalue
    (:Is%20Valid
      (EventDispatchers|AssignPowerOff _returnvalue (delegate Custom|OnPowerOff)))))

(fn ConstructionScript)

(fn GetState
  (return (Variables|Default|GetOn)))