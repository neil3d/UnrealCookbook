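; BP_MyGameMode is a game mode that tracks which pickup types the player has collected.
; PickupItem adds the given type to a set, so duplicates count once, and prints progress as collected over the total enum entry count.
; HasAllItems reports whether the set size equals the number of entries in the pickup enum.
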(fn ConstructionScript
  (|CallParentFunction))

(fn PickupItem
  (params (PickupType :type EMyPickupType%20Enum :default "NewEnumerator0"))
  (bind _mypickupset (Variables|Default|GetMyPickupSet))
  (Utilities|Set|Add _mypickupset PickupType)
  (Development|PrintText (Utilities|Text|FormatText "Pickup {0}/{1}" (Utilities|Set|Length _mypickupset) (|GetNumEnumEntries))))

(fn HasAllItems
  (return (== (Utilities|Set|Length (Variables|Default|GetMyPickupSet)) (|GetNumEnumEntries))))