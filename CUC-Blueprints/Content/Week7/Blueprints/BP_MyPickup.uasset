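; BP_MyPickup is a collectible pickup that can be a coin, cupcake or health item, selected by MyType.
; The construction script sets the matching static mesh, and Tick bobs it vertically with a time-based sine wave.
; Any actor overlap reports the type to BP_MyGameMode through PickupItem, then destroys the pickup, even if the game mode cast fails.
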(event EventTick
  (params (DeltaSeconds :type Float%20%28single-precision%29))
  (Transformation|SetRelativeLocation (Variables|Default|GetSM_Pickup) (Math|Vector|MakeVector 0.0 0.0 (* (Math|Trig|Sin(Radians) (* (Utilities|Time|GetTimeSeconds) 3.0)) 2e+01)) false false))

(event Collision|EventActorBeginOverlap
  (params (OtherActor :type Actor%20Object%20Reference))
  (Utilities|FlowControl|Sequence
    (:then_0
      (bind _asbp_my_game_mode (Utilities|Casting|CastToBP_MyGameMode (Game|GetGameMode)))
      (Default|PickupItem _asbp_my_game_mode (Variables|Default|GetMyType)))
    (:then_1
      (Actor|DestroyActor))))

(fn ConstructionScript
  (bind _sm_pickup (Variables|Default|GetSM_Pickup))
  (switch Utilities|FlowControl|Switch|SwitchonEMyPickupType (Variables|Default|GetMyType)
    (:NewEnumerator0
      (Components|StaticMesh|SetStaticMesh _sm_pickup "/Game/DemoRoom/Meshes/SM_Pickup_Coin.SM_Pickup_Coin"))
    (:NewEnumerator1
      (Components|StaticMesh|SetStaticMesh _sm_pickup "/Game/DemoRoom/Meshes/SM_Pickup_Cupcake.SM_Pickup_Cupcake"))
    (:NewEnumerator2
      (Components|StaticMesh|SetStaticMesh _sm_pickup "/Game/DemoRoom/Meshes/SM_Pickup_Health.SM_Pickup_Health"))))