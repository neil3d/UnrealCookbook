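; BP_MyDoor is a door that swings open when something overlaps its Box trigger and snaps shut when the overlap ends.
; A locked door opens only if BP_MyGameMode reports that all items are held, while an unlocked door always opens.
; The construction script colors the mesh red when locked and orange otherwise.
; Rotation is set instantly without animation, and each open or close prints a message.
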(event OnComponentBeginOverlap(Box)
  (params (OverlappedComponent :type Primitive%20Component%20Object%20Reference) (OtherActor :type Actor%20Object%20Reference) (OtherComp :type Primitive%20Component%20Object%20Reference) (OtherBodyIndex :type Integer) (bFromSweep :type Boolean) (SweepResult :type Hit%20Result%20Structure%20%28by%20ref%29))
  (if (Variables|Default|GetLocked)
    (bind _asbp_my_game_mode (Utilities|Casting|CastToBP_MyGameMode (Game|GetGameMode)))
    (bind _result (Default|HasAllItems _asbp_my_game_mode))
    (if _result
      (Transformation|SetRelativeRotation (Variables|Default|GetSM_Door) "0,110.000000, 0" false false :!label _label)
      (Development|PrintString "Door opened"))
    (else
      (goto _label))))

(event OnComponentEndOverlap(Box)
  (params (OverlappedComponent :type Primitive%20Component%20Object%20Reference) (OtherActor :type Actor%20Object%20Reference) (OtherComp :type Primitive%20Component%20Object%20Reference) (OtherBodyIndex :type Integer))
  (Transformation|SetRelativeRotation (Variables|Default|GetSM_Door) "0,0.000000, 0" false false)
  (Development|PrintString "Door closed"))

(fn ConstructionScript
  (bind _sm_door (Variables|Default|GetSM_Door))
  (if (Variables|Default|GetLocked)
    (Rendering|Material|SetMaterial _sm_door 0 "/Game/DemoRoom/Materials/M_Red_Shiny.M_Red_Shiny")
    (else
      (Rendering|Material|SetMaterial _sm_door 0 "/Game/DemoRoom/Materials/M_Orange_Shiny.M_Orange_Shiny"))))