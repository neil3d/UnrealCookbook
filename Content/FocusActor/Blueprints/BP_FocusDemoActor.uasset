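; BP_FocusDemoActor is a demo actor that shows a floating info text while it has focus.
; It hides the text on BeginPlay, then the focus interface events OnFocus and LostFocus toggle its visibility.
; The construction script sets the text from InfoText, cancels the actor's scale so the text keeps its size, and places it at the top of the static mesh's local bounds.
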(event EventBeginPlay
  ;[1 1 1] Hide Info Text at Beginning
  (Rendering|SetVisibility (Variables|Default|GetScreenTextRender) false false))

(event EventOnFocus
  ;[1 1 1] FoucsAction Interface
  (Rendering|SetVisibility (Variables|Default|GetScreenTextRender) true false))

(event EventLostFocus
  ;[1 1 1] FoucsAction Interface
  (Rendering|SetVisibility (Variables|Default|GetScreenTextRender) false false))

(fn ConstructionScript
  (bind _screentextrender (Variables|Default|GetScreenTextRender))
  ;[1 1 1] Init Text Box
  (Transformation|SetRelativeScale3D _screentextrender (/ "1.000000,1.000000,1.000000" (Transformation|GetActorScale3D)))
  (Transformation|SetRelativeLocation _screentextrender (Math|Vector|MakeVector 0.0 0.0 (.Z (Math|Vector|BreakVector (.Max (Components|StaticMesh|GetLocalBounds (Variables|Debug|GetStaticMeshComponent)))))) false false)
  (Rendering|Components|TextRender|SetText _screentextrender (Variables|FocusActorDemo|GetInfoText)))