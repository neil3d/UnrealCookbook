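; BP_LoadDataAsset is a demo actor that asynchronously loads a quest data asset by its asset ID when play begins.
; After a short delay, Async Load Asset resolves QuestAssetID and the result is cast to QuestDataAsset.
; On success it prints the quest set name and each quest name from QuestArray to the screen, otherwise it prints a failure message.
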(event EventBeginPlay
  (Utilities|FlowControl|Delay 0.5)
  (bind _object (Utilities|AsyncLoadAsset (Variables|Default|GetQuestAssetID)))
  (Development|PrintString "Load Asset Completed" true true "(R=1.000000,G=0.242666,B=0.166153,A=1.000000)" 2e+01)
  (bind _asquest_data_asset (Utilities|Casting|CastToQuestDataAsset _object)
    (:then
      (Development|PrintString (Variables|/Script/UnrealCookBook.QuestDataAsset|GetQuestSetName _asquest_data_asset) true true "(R=0.000000,G=0.660000,B=1.000000,A=1.000000)" 2e+01)
      (for _array_element (Variables|/Script/UnrealCookBook.QuestDataAsset|GetQuestArray _asquest_data_asset)
        (Development|PrintString (.QuestName (Utilities|Struct|BreakQuestDef _array_element)) true true "(R=0.000000,G=0.660000,B=1.000000,A=1.000000)" 2e+01)))
    (:CastFailed
      (Development|PrintString "Load QuestDataSAsset FAILED!"))))

(fn ConstructionScript)