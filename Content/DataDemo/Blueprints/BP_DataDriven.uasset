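; BP_DataDriven is a demo actor that reads the Tab_ItemDef item data table, which a comment marks as CSV-sourced.
; On BeginPlay it prints a header, then loops over every row name and looks up each row.
; Each found row's name, damage, price and description are formatted into one line and printed on screen.
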(event EventBeginPlay
  ;[1 1 1] Load a CSV Data Table
  (Development|PrintString "Table Content:" true true "(R=0.000000,G=0.660000,B=1.000000,A=1.000000)" 2e+01)
  (bind _outrownames (DataTable|GetDataTableRowNames "/Game/DataDemo/Data/Tab_ItemDef.Tab_ItemDef"))
  (for _array_element _outrownames
    (bind _returnvalue (Utilities|GetDataTableRow "/Game/DataDemo/Data/Tab_ItemDef.Tab_ItemDef" _array_element)
      (:then
        (Development|PrintString (Utilities|String|ToString(Text) (Utilities|Text|FormatText "Item Name={0} Damage={1} Price={2} Desc:{3}" (Utilities|Text|ToText(Name) (.Name (Utilities|Struct|BreakItemDef _returnvalue))) (Utilities|Text|ToText(Float) (.Damage (Utilities|Struct|BreakItemDef _returnvalue)) "HalfToEven") (Utilities|Text|ToText(Float) (.Price (Utilities|Struct|BreakItemDef _returnvalue)) "HalfToEven") (.Desc (Utilities|Struct|BreakItemDef _returnvalue)))) true true "(R=0.000000,G=0.660000,B=1.000000,A=1.000000)" 2e+01)))))

(fn ConstructionScript)